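; BP_LevelBackup holds level camera logic, apparently a backup, for viewing and tracking the BP_PlayerCube pawn.
; One custom event switches player 0's view target to a camera actor, and another casts the player pawn to BP_PlayerCube.
; RotateCamera turns an actor to face that cube using a look-at rotation.
; Several target references are unresolved, and a blended view-target switch is left unconnected.
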(event Custom|RotateCamera
  ;[1 1 1] Comment
  (Transformation|SetActorRotation "Literal" (Math|Rotator|FindLookatRotation (Transformation|GetActorLocation "Literal") (Transformation|GetActorLocation (stale Custom|CustomEvent_1 _asbp_player_cube)))))

(event Custom|CustomEvent
  ;[1 1 1] Set cameraActor as level camera
  (Game|Player|SetViewTargetwithBlend (Game|GetPlayerController 0) "Literal" 0.0 "VTBlend_Linear" 0.0 false))

(event Custom|CustomEvent_1
  (params (DeltaSeconds :type Float%20%28single-precision%29))
  ;[1 1 1] Comment
  (bind _asbp_player_cube (Utilities|Casting|CastToBP_PlayerCube (Game|Player|GetPlayerPawn 0))))