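; BP_SaveGame is a save game Blueprint that persists the player's high score and contains its own load and save logic.
; LoadHighScore reads the slot named by SlotName, casts it to BP_SaveGame and copies the stored HighScore into its own variable.
; SaveHighScore refreshes that value first, then writes a newly created save object to the slot only if the new score is higher.
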(event Custom|SaveHighScore
  (params (Score :type Integer))
  (CallFunction|LoadHighScore)
  (bind _returnvalue (SaveGame|CreateSaveGameObject "BP_SaveGame_C"))
  (if (> Score (Variables|Default|GetHighScore))
    (Variables|BP_SaveGame_C|SetHighScore _returnvalue Score)
    (SaveGame|SaveGametoSlot _returnvalue (Variables|Default|GetSlotName))))

(event Custom|LoadHighScore
  (bind _returnvalue (SaveGame|LoadGamefromSlot (Variables|Default|GetSlotName)))
  (bind _asbp_save_game (Utilities|Casting|CastToBP_SaveGame _returnvalue))
  (Variables|Default|SetHighScore (Variables|BP_SaveGame_C|GetHighScore _asbp_save_game)))