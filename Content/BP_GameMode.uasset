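; BP_GameMode is a game mode that creates the main scene UI and tracks the current points and height.
; On BeginPlay it creates a BP_MainSceneUI widget, stores it in CurrentUi and adds it to the viewport.
; UpdatePoints increments the point count and UpdateHeight stores the given height, each writing the new value straight into the widget's matching variable.
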(event Custom|UpdateHeight
  (params (Height :type Float%20%28single-precision%29))
  ;[1 1 1] UpdateHeightTextbox
  (bind _output_get (Variables|Default|SetCurrentHeight Height))
  (Variables|/Game/BP_MainSceneUI.BP_MainSceneUI_C|SetHeight (Variables|Default|GetCurrentUi) _output_get))

(event Custom|Update%20Points
  ;[1 1 1] UpdatePointsTextbox
  (bind _output_get (Variables|Default|SetCurrentPoints (+ 1 (Variables|Default|GetCurrentPoints))))
  (Variables|/Game/BP_MainSceneUI.BP_MainSceneUI_C|SetPoints (Variables|Default|GetCurrentUi) _output_get))

(event EventBeginPlay
  ;[1 1 1] Add Ui to view
  (bind _returnvalue (UserInterface|CreateWidget "/Game/BP_MainSceneUI.BP_MainSceneUI_C"))
  (bind _output_get (Variables|Default|SetCurrentUi _returnvalue))
  (UserInterface|Viewport|AddtoViewport _output_get 0))

(fn ConstructionScript)